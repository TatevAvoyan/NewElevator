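; BP_InteractObject is an interactable object, filed as a parent Blueprint, that can be highlighted and picked up.
; FocusBegin and FocusEnd toggle the StaticMesh's custom depth rendering to mark focus.
; Use flips Active and applies it to actor tick, collision and visibility.
; Use returns the actor itself for the inventory; a null return signals an action that adds no item.
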(fn ConstructionScript)

(fn FocusBegin
  (Rendering|SetRenderCustomDepth (Variables|Default|GetStaticMesh) true))

(fn FocusEnd
  (Rendering|SetRenderCustomDepth (Variables|Default|GetStaticMesh) false))

(fn Use
  (bind _self self)
  (bind _output_get (Variables|Default|SetActive (not (Variables|Default|GetActive))))
  (Actor|Tick|SetActorTickEnabled _self _output_get)
  (Collision|SetActorEnableCollision _self _output_get)
  (Rendering|SetActorHiddenInGame _self (not (Variables|Default|GetActive)))
  ;[1 1 1] Return null to do something, without adding item to inventory
  (return _self))